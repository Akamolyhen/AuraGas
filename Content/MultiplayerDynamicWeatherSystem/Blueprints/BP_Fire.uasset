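; BP_Fire is a fire actor in the multiplayer weather system that goes out in rain unless it is sheltered.
; When OnRain signals rain, an upward Visibility line trace from just above the actor checks for overhead cover.
; With no hit, it disables the Flames and Smoke particle emitters and mutes the audio.
; When rain stops, it re-enables both emitters and restores full volume.
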(event `/Game/MultiplayerDynamicWeatherSystem/Blueprints/BI_MultiplayerDynamicWeatherSystem.On Rain`
  (params (`Raining?` :type Boolean))
  (bind _returnvalue (`self.K2_GetActorLocation`))
  (bind _fire (`self.Fire`))
  (bind _audio (`self.Audio`))
  (bind _fire_2 (`self.Fire`))
  (if `Raining?`
    ;[0 0 0] Can disappear
    (bind (_outhit _returnvalue_2) (`KismetSystemLibrary.LineTraceSingle` (+ _returnvalue (0.0 0.0 25.0)) (+ _returnvalue (0.0 0.0 10000.0)) "TraceTypeQuery1"))
    (if (not _returnvalue_2)
      ;[1 1 1] Stop Emitter
      (`ParticleSystemComponent.SetEmitterEnable` _fire_2 "Flames" false)
      (`ParticleSystemComponent.SetEmitterEnable` _fire_2 "Smoke" false)
      (`AudioComponent.SetVolumeMultiplier` _audio 0.0))
    (else
      ;[1 1 1] Start Emitter
      (`ParticleSystemComponent.SetEmitterEnable` _fire "Flames" true)
      (`ParticleSystemComponent.SetEmitterEnable` _fire "Smoke" true)
      (`AudioComponent.SetVolumeMultiplier` _audio 1.0))))

(fn `UserConstructionScript`)