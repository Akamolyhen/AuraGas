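; Automatic double sliding door that opens when something overlaps its Box trigger and closes when an overlap ends.
; Begin overlap plays the MoveLeftDoor timeline and end overlap reverses it, with no filter on the overlapping actor.
; Despite its name, the timeline drives both panels, with a separate track setting each one's relative Y while keeping X and Z.
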(event `self.Box.OnComponentBeginOverlap`
  (params (OverlappedComponent :type "PrimitiveComponent Object Reference") (OtherActor :type "Actor Object Reference") (OtherComp :type "PrimitiveComponent Object Reference") (OtherBodyIndex :type Integer) (bFromSweep :type Boolean) (SweepResult :type "HitResult Structure (by ref)"))
  (bind (_direction _leftdoormoveline _rightdoormoveline) (`Timeline|MoveLeftDoor` :!label _label)
    (:`Update`
      (`|ExecutionSequence`
        (:`then_0`
          (`self.Relative Move LeftDoor` _leftdoormoveline))
        (:`then_1`
          (`self.Relative Move RightDoor` _rightdoormoveline))))))

(event `self.Box.OnComponentEndOverlap`
  (params (OverlappedComponent :type "PrimitiveComponent Object Reference") (OtherActor :type "Actor Object Reference") (OtherComp :type "PrimitiveComponent Object Reference") (OtherBodyIndex :type Integer))
  (goto _label :!via `Reverse`))

(fn `Relative Move LeftDoor`
  (params (RelativeMove :type "Float (double-precision)"))
  (bind _door_left (`self.door_Left`))
  (bind (_relativelocation_x _relativelocation_y _relativelocation_z) (`KismetMathLibrary.BreakVector` (`SceneComponent.RelativeLocation` _door_left)))
  (`SceneComponent.K2_SetRelativeLocation` _door_left (`KismetMathLibrary.MakeVector` _relativelocation_x RelativeMove _relativelocation_z) false false))

(fn `Relative Move RightDoor`
  (params (RelativeMove :type "Float (double-precision)"))
  (bind _door_right (`self.door_Right`))
  (bind (_relativelocation_x _relativelocation_y _relativelocation_z) (`KismetMathLibrary.BreakVector` (`SceneComponent.RelativeLocation` _door_right)))
  (`SceneComponent.K2_SetRelativeLocation` _door_right (`KismetMathLibrary.MakeVector` _relativelocation_x RelativeMove _relativelocation_z) false false))

(fn `UserConstructionScript`)