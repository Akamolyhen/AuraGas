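; Hit-reaction gameplay ability that plays a flinch montage on goblin slingshot and spear avatars.
; On activation it applies GE_HitReact to the owner, then tries both goblin casts, each leading to the montage supplied by CombatInterface.
; Montage completion, interruption or cancellation removes the effect by its stored handle and ends the ability.
; Avatars failing both casts never reach that cleanup; the cached skeletal mesh only feeds disconnected code.
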(event `self.K2_ActivateAbility`
  (bind _returnvalue (`self.BP_ApplyGameplayEffectToOwner` "/Game/Blueprints/AbilitySystem/GameplayEffects/GE_HitReact.GE_HitReact_C"))
  (set `self.ActiveGE_HitReact` _returnvalue)
  (`|ExecutionSequence`
    (:`then_0`
      (bind _asbp_goblin_slingshot (cast `/Game/Blueprints/Character/Goblin/Goblin_Slingshot/BP_Goblin_Slingshot` (`self.GetAvatarActorFromActorInfo`)))
      (set `self.In Skeletal Mesh Component` (`Character.Mesh` _asbp_goblin_slingshot)))
    (:`then_1`
      (bind _asbp_goblin_spear (cast `/Game/Blueprints/Character/Goblin/Goblin_Spear/BP_Goblin_Spear` (`self.GetAvatarActorFromActorInfo`)))
      (set `self.In Skeletal Mesh Component` (`Character.Mesh` _asbp_goblin_spear))))
  (bind _ascombat_interface (cast `CombatInterface` (`self.GetAvatarActorFromActorInfo`)))
  (bind _returnvalue_2 (`CombatInterface.GetHitReactMontage` _ascombat_interface))
  (`AbilityTask_PlayMontageAndWait.CreatePlayMontageAndWaitProxy` "None" _returnvalue_2
    (:`OnCompleted`
      _)
    (:`OnInterrupted`
      _)
    (:`OnCancelled`
      _))
  (`self.BP_RemoveGameplayEffectFromOwnerWithHandle` (`self.ActiveGE_HitReact`))
  (`self.K2_EndAbility`))